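; Base player character with camera-relative movement, health with a widget bar, stat passives, an abilities component and one-time death that notifies the game mode.
; Character class data, currently a hardcoded default on BeginPlay, replicates through OnRep functions that set the starting ability and skeletal mesh.
; Pause requests go through server and multicast events that fake pausing with near-zero global time dilation, with the game mode gating unpause unless overridden.
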(event Custom|SetupWidgets
  (CharacterSetup|CreateHealthWidget))

(event Custom|S_SetCharacterData
  (params (CharacterData :type ST%20Available%20Characters%20Structure))
  (Variables|CharacterSetup|SetCharacter CharacterData))

(event Custom|Death
  (Default|InvalidateTimers (Variables|Default|GetBP_Abilities_Component))
  (Input|DisableInput (Variables|CharacterSetup|GetLocal%20Player%20Controller))
  (Animation|PlayAnimMontage "/Game/Anims/KB_HighKO_R1_Montage.KB_HighKO_R1_Montage" 1.0 "None")
  (Collision|SetCollisionResponsetoChannel (Variables|Collision|GetCapsuleComponent) "ECC_GameTraceChannel1" "ECR_Ignore")
  (Collision|SetCollisionResponsetoChannel (Variables|Collision|GetCapsuleComponent) "ECC_Pawn" "ECR_Ignore"))

(event Custom|S_SetCharacterMesh
  (params (SK :type Skeletal%20Mesh%20Object%20Reference))
  (Variables|CharacterSetup|SetCharSK SK))

(event Custom|UpdateHealthBar
  (params (Percent :type Float%20%28double-precision%29))
  (bind _healthbarwidgetreference (Variables|Character|GetHealthBarWidgetReference)
    (:then
      (Progress|SetPercent (Variables|/Game/UI/WB_HealthBar.WB_HealthBar_C|GetProgressBar_128 _healthbarwidgetreference) Percent))
    (:else)))

(event Game|Damage|EventAnyDamage
  (params (Damage :type Float%20%28single-precision%29) (DamageType :type Damage%20Type%20Object%20Reference) (InstigatedBy :type Controller%20Object%20Reference) (DamageCauser :type Actor%20Object%20Reference))
  (bind _output_get (Variables|Character|SetCurrentHealth (- (Variables|Character|GetCurrentHealth) Damage)))
  (CallFunction|UpdateHealthBar (/ (Variables|Character|GetCurrentHealth) (Variables|Character|GetMaxHealth)))
  (if (<= _output_get 0.0)
    (Utilities|FlowControl|DoOnce false
      (:Completed
        (Variables|Character|SetIsDead true)
        (CallFunction|Death)
        (Default|OnPlayerDeath (Variables|CharacterSetup|GetGM_Interface))))))

(event EventRestoreHealth
  (params (Amount :type Float%20%28double-precision%29))
  (Variables|Character|SetCurrentHealth (Math|Float|Clamp(Float) (+ (Variables|Character|GetCurrentHealth) Amount) 0.0 (Variables|Character|GetMaxHealth)))
  (CallFunction|UpdateHealthBar (/ (Variables|Character|GetCurrentHealth) (Variables|Character|GetMaxHealth))))

(event EventUpdateCharacterClass
  (params (Character :type ST%20Available%20Characters%20Structure))
  (CallFunction|SSetCharacterData Character))

(event EventAdjustPassive
  (params (Stat :type E_PassiveAbilities%20Enum :default "NewEnumerator0") (MultiplicationAmount :type Float%20%28double-precision%29))
  (bind _charactermovement (Variables|Character|GetCharacterMovement))
  (switch Utilities|FlowControl|Switch|SwitchonE_PassiveAbilities Stat
    (:NewEnumerator1
      (bind _output_get (Variables|Character|SetMaxHealth (* (Variables|Character|GetMaxHealth) MultiplicationAmount)))
      (CallFunction|RestoreHealth (* _output_get 0.1)))
    (:NewEnumerator3
      (Variables|/Script/Engine.CharacterMovementComponent|SetMaxWalkSpeed _charactermovement (* (Variables|/Script/Engine.CharacterMovementComponent|GetMaxWalkSpeed _charactermovement) MultiplicationAmount)))))

(event EventBeginPlay
  (CharacterSetup|SetupReferences)
  (CharacterSetup|LoadLastCharacterClass)
  (Utilities|FlowControl|Delay 1.0)
  (CallFunction|SetupWidgets))

(event EventSetupHealthWidget
  (CallFunction|SetupWidgets))

(event Input|AxisEvents|InputAxisMoveForward/Backward
  (params (AxisValue :type Float%20%28single-precision%29))
  (Pawn|Input|AddMovementInput (Math|Vector|GetForwardVector (Math|Rotator|MakeRotator 0.0 0.0 (.yaw (Transformation|GetWorldRotation (Variables|Default|GetCamera))))) AxisValue false))

(event Input|AxisEvents|InputAxisMoveRight/Left
  (params (AxisValue :type Float%20%28single-precision%29))
  (Pawn|Input|AddMovementInput (Math|Vector|GetRightVector (Math|Rotator|MakeRotator 0.0 0.0 (.yaw (Transformation|GetWorldRotation (Variables|Default|GetCamera))))) AxisValue false))

(fn ConstructionScript)

(fn CreateHealthWidget
  (bind _returnvalue (UserInterface|CreateWidget "/Game/UI/WB_HealthBar.WB_HealthBar_C"))
  (bind _output_get (Variables|Character|SetHealthBarWidgetReference _returnvalue))
  (UserInterface|SetWidget (Variables|Default|GetHealthWidget) _output_get)
  (CallFunction|UpdateHealthBar (/ (Variables|Character|GetCurrentHealth) (Variables|Character|GetMaxHealth))))

(fn SetupReferences
  (bind _asbp_sr_player_controller (Utilities|Casting|CastToBP_SR_PlayerController (Pawn|GetController)))
  (Variables|CharacterSetup|SetLocal%20Player%20Controller _asbp_sr_player_controller))

(fn LoadLastCharacterClass
  (CallFunction|SSetCharacterData (Utilities|Struct|MakeST_AvailableCharacters "NewEnumerator0" 0 false 0 "Description of Character" "Arlo")))

(fn SetupDispatchers)

(fn ORonRepCharacterClass)

(fn OnRepCharacter
  (bind _character (Variables|CharacterSetup|GetCharacter))
  (bind (_startingability _charactersk) (Utilities|Struct|BreakST_AvailableCharacters _character))
  (CallFunction|ORonRepCharacterClass)
  (Variables|CharacterSetup|SetStartingAbility _startingability)
  (CallFunction|SSetCharacterMesh _charactersk))

(fn OnRepCharSK
  (bind _charsk (Variables|CharacterSetup|GetCharSK)
    (:then
      (Components|SkinnedMesh|SetSkinnedAssetandUpdate (Variables|Character|GetMesh) _charsk false))
    (:else)))

(event Custom|OnPause
  (params (Pause :type Boolean) (Override :type Boolean))
  (CallFunction|SPause Pause Override))

(event Custom|S_Pause
  (params (Pause :type Boolean) (Override :type Boolean))
  (bind _returnvalue (Game|GetGameMode))
  (if Pause
    (CallFunction|MCPause Pause)
    (Utilities|Time|SetGlobalTimeDilation 0.0001)
    (bind _asbp_sr_game_mode (Utilities|Casting|CastToBP_SR_GameMode (Game|GetGameMode)))
    (Variables|/Game/Gameplay/BP_SR_GameMode.BP_SR_GameMode_C|SetGameIsPaused _asbp_sr_game_mode true)
    (elif Override
      (bind _asbp_sr_game_mode_2 (Utilities|Casting|CastToBP_SR_GameMode _returnvalue))
      (Default|ResetPauseCount _asbp_sr_game_mode_2)
      (CallFunction|MCPause Pause :!label _label)
      (Utilities|Time|SetGlobalTimeDilation 1.0)
      (bind _asbp_sr_game_mode_3 (Utilities|Casting|CastToBP_SR_GameMode (Game|GetGameMode)))
      (Variables|/Game/Gameplay/BP_SR_GameMode.BP_SR_GameMode_C|SetGameIsPaused _asbp_sr_game_mode_3 false)
      (else
        (bind _asbp_sr_game_mode_4 (Utilities|Casting|CastToBP_SR_GameMode _returnvalue))
        (bind _shouldresume (Default|CheckPlayersforPause _asbp_sr_game_mode_4))
        (if _shouldresume
          (goto _label))))))

(event Custom|MC_Pause
  (params (Pause :type Boolean))
  (if Pause
    (Utilities|Time|SetGlobalTimeDilation 0.0001)
    (else
      (Utilities|Time|SetGlobalTimeDilation 1.0))))

(event EventPause
  (params (Pause :type Boolean) (Override :type Boolean))
  (CallFunction|OnPause Pause Override))

(fn GetAbilityComponent
  (return (Variables|Default|GetBP_Abilities_Component)))

(fn GetAbilitySphere
  (return (Variables|Default|GetAbilitySphere)))

(fn GetCharacter
  (return self))

(fn IsAlive
  (return (not (Variables|Character|GetIsDead))))