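; BP_HPBall is a health orb pickup that restores health to the character that picks it up.
; DoPickupAction sends a RestoreHealth message to the character with HealthAmount.
; PickupEffects attaches a scaled-up orb particle burst to the passed actor's root and plays a health sound at the orb's location.
; Overlap detection and the triggering of both events are not in this graph, whose BeginPlay, overlap and Tick nodes are disabled.
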(event EventBeginPlay
  (|CallParentFunction) ; This node is disabled and will not be called.\nDrag off pins to build functionality.
)

(event Collision|EventActorBeginOverlap
  (params (OtherActor :type Actor%20Object%20Reference))
  (|CallParentFunction OtherActor) ; This node is disabled and will not be called.\nDrag off pins to build functionality.
)

(event EventTick
  (params (DeltaSeconds :type Float%20%28single-precision%29))
  (|CallParentFunction DeltaSeconds) ; This node is disabled and will not be called.\nDrag off pins to build functionality.
)

(event EventDoPickupAction
  (params (Character :type Actor%20Object%20Reference))
  ;[0.1094 0.1094 0.1094] Restore character Health
  (Class|ICharacterManager|RestoreHealth(Message) Character (Variables|Default|GetHealthAmount)))

(event EventPickupEffects
  (params (InActor :type Actor%20Object%20Reference))
  (Effects|SpawnEmitterAttached "/Game/VFX/FX_Archive/P_HealthOrb_Pickup.P_HealthOrb_Pickup" (Variables|/Script/Engine.Actor|GetRootComponent InActor) "None" "0, 0, 0" "0, 0, 0" "2.000000,2.000000,2.000000")
  (Audio|PlaySoundatLocation "/Game/Sound/Character/Cue_Health.Cue_Health" (Transformation|GetActorLocation) "0, 0, 0" 1.0 1.0 0.0 0 0 0 0))

(fn ConstructionScript
  (|CallParentFunction))